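; Manager component that registers and controls points of interest (POIs) in a level with a BP_ViewPawn camera.
; On BeginPlay it caches the pawn and indexes all BP_POIbase actors into a nested map by group, then name.
; Functions find POIs, handle selection, switch widget types, and show or hide groups with optional delayed animation.
; It also exposes pawn arm state and applies a POI's zoom range to the spring arm limits.
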(event Custom|ChangeGroupsPOItype
  (params (Group :type String) (TypeIndex :type Integer))
  (bind _output_get (Variables|Default|SetIconViewType TypeIndex))
  (bind _pois (功能|FuncFindGroupPOIs Group))
  (Class|BPIPOIInterface|ChangePOItypes(Message) _pois _output_get))

(event Custom|ChangePOIHidAni
  (params (Group :type String) (Hid :type Boolean))
  (bind _output_get (Variables|Default|SetHid Hid))
  (bind _pois (功能|FuncFindGroupPOIs Group))
  (Class|BPIPOIInterface|ChangePOIdata(Message) _pois _output_get))

(event EventBeginPlay
  (Utilities|FlowControl|Sequence
    (:then_0
      (bind _asbp_view_pawn (Utilities|Casting|CastToBP_ViewPawn (Game|Player|GetPlayerPawn 0))
        (:then
          (Variables|Default|SetPOI_Pawn _asbp_view_pawn))
        (:CastFailed
          (Development|PrintString "Pawn不是插件指定的pawn"))))
    (:then_1
      (bind _outactors (Actor|GetAllActorsOfClass "/POItools_Beta01/POItools/POI/BP_POIbase.BP_POIbase_C"))
      (for _array_element _outactors
        (CallFunction|AddPOI _array_element)))))

(event EventTick
  (params (DeltaSeconds :type Float%20%28single-precision%29)))

(fn AddPOI
  (params (POI :type BP%20PO%20Ibase%20Object%20Reference))
  (bind _poi_groupmes (Variables|Default|GetPOI_GroupMes))
  (bind _poi_group (Variables|/POItools_Beta01/POItools/POI/BP_POIbase.BP_POIbase_C|GetPOI_Group POI))
  (bind _mymessage (Variables|/POItools_Beta01/POItools/POI/BP_POIbase.BP_POIbase_C|GetMyMessage POI))
  (bind (_value _returnvalue) (Utilities|Map|Find _poi_groupmes _poi_group))
  (if _returnvalue
    (bind _output_get (LocalVariables|SetNewLocalMes (Utilities|Struct|BreakStr_POIDictionary _value)))
    (Utilities|Map|Add _output_get (.name _mymessage) POI)
    (Utilities|Map|Add _poi_groupmes _poi_group (Utilities|Struct|MakeStr_POIDictionary (LocalVariables|GetNewLocalMes)))
    (else
      (Utilities|Map|Add _poi_groupmes _poi_group (Utilities|Struct|MakeStr_POIDictionary (Utilities|Map|MakeMap (.name _mymessage) POI))))))

(fn ManagerSelectPOI
  (params (SelectedPOI :type BP%20PO%20Ibase%20Object%20Reference))
  (bind _selectedpoi (Variables|Default|GetSelectedPOI)
    (:then
      (Class|BPIPOIInterface|EUnSelected(Message) _selectedpoi))
    (:else
      _))
  (bind _output_get (Variables|Default|SetSelectedPOI SelectedPOI))
  (Class|BPIPOIInterface|ESelected(Message) _output_get))

(fn FuncFindPOI
  (params (Group :type String) (Name :type String))
  (bind _poi_groupmes (Variables|Default|GetPOI_GroupMes))
  (bind (_value _returnvalue) (Utilities|Map|Find _poi_groupmes Group))
  (bind _poi_dic (Utilities|Struct|BreakStr_POIDictionary _value))
  (bind (_value_2 _returnvalue_2) (Utilities|Map|Find _poi_dic Name))
  (if (Utilities|Array|IsEmpty Group)
    (bind _values (Utilities|Map|Values _poi_groupmes))
    (bind _array_element (Utilities|Array|ForEachLoopwithBreak _values)
      (:LoopBody
        (if (.ReturnValue (Utilities|Map|Find (Utilities|Struct|BreakStr_POIDictionary _array_element) Name))
          (bind _output_get (LocalVariables|SetLocalPOI (.Value (Utilities|Map|Find (Utilities|Struct|BreakStr_POIDictionary _array_element) Name))))
          (return _output_get true)))
      (:Completed
        (LocalVariables|GetLocalPOI
          (:then)
          (:else
            (return 0 false)))))
    (elif _returnvalue
      (return _value_2 _returnvalue_2)
      (else
        (return 0 false)))))

(fn FuncFindGroupPOIs
  (params (Group :type String%20%28by%20ref%29))
  (bind _values (Utilities|Map|Values (Utilities|Struct|BreakStr_POIDictionary (.Value (Utilities|Map|Find (Variables|Default|GetPOI_GroupMes) Group)))))
  (return _values))

(fn FuncSetGroupPOIVisit
  (params (Group :type String) (Visit :type Boolean) (UseAni :type Boolean) (Delay :type Float%20%28double-precision%29))
  (bind _iconviewtype (Variables|Default|GetIconViewType))
  (bind _pois (功能|FuncFindGroupPOIs Group))
  (for _array_element _pois
    (if (!= (Variables|/POItools_Beta01/POItools/POI/BP_POIbase.BP_POIbase_C|GetisVisited _array_element) Visit)
      (bind _output_get (Variables|/POItools_Beta01/POItools/POI/BP_POIbase.BP_POIbase_C|SetisVisited _array_element Visit))
      (if (== (Variables|/POItools_Beta01/POItools/POI/BP_POIbase.BP_POIbase_C|GetWidgetTypeIndex _array_element) _iconviewtype) ; 类型不等时，先同步类型
        _
        (else
          (Default|SetWidgetTypeandUpdate _array_element _iconviewtype)))
      (if UseAni
        (Default|SetPOIVisit _array_element Visit Delay)
        (else
          (Rendering|SetActorHiddenInGame _array_element (not _output_get)))))))

(fn FuncShowOneGroupPOI
  (params (Group :type String) (UseAni :type Boolean) (HidDelay :type Float%20%28double-precision%29) (ShowDelay :type Float%20%28double-precision%29))
  (bind _keys (Utilities|Map|Keys (Variables|Default|GetPOI_GroupMes)))
  (for _array_element _keys
    (功能|FuncSetGroupPOIVisit _array_element (Utilities|Enum|Equal(Enum) _array_element Group) UseAni (select (Utilities|Enum|Equal(Enum) _array_element Group) ShowDelay HidDelay))))

(fn FuncSetPoiCameraRange
  (params (Group :type String) (Name :type String))
  (bind (_value _find) (功能|FuncFindPOI Group Name)) ; 重设缩放范围和鼠标平移速度
  (if _find
    (CallFunction|UpdataPawnCameraRange (Variables|/POItools_Beta01/POItools/POI/BP_POIbase.BP_POIbase_C|GetPOI_CameraRange _value))
    (return _value)))

(fn GetPawnIsMoving
  (bind _poi_pawn (Variables|Default|GetPOI_Pawn)
    (:then
      (return (not (Variables|/POItools_Beta01/POItools/Gameplay/BP_ViewPawn.BP_ViewPawn_C|GetisCloseArm _poi_pawn))))
    (:else
      (return false))))

(fn GetpawnArmLength
  (bind _poi_pawn (Variables|Default|GetPOI_Pawn)
    (:then
      (return (Variables|/Script/Engine.SpringArmComponent|GetTargetArmLength (Variables|/POItools_Beta01/POItools/Gameplay/BP_ViewPawn.BP_ViewPawn_C|GetSpringArm _poi_pawn))))
    (:else)))

(fn GetPawnArmMaximum
  (bind _poi_pawn (Variables|Default|GetPOI_Pawn)
    (:then
      (return (Variables|/POItools_Beta01/POItools/Gameplay/BP_ViewPawn.BP_ViewPawn_C|GetSpringArm_Length_Min _poi_pawn) (Variables|/POItools_Beta01/POItools/Gameplay/BP_ViewPawn.BP_ViewPawn_C|GetSpringArm_Length_Max _poi_pawn)))
    (:else)))

(fn UpdataPawnCameraRange
  (params (CameraRange :type Vector%202D%20Structure))
  (bind (_x _y) (Math|Vector2D|BreakVector2D CameraRange))
  (bind _poi_pawn (Variables|Default|GetPOI_Pawn)
    (:then
      (Variables|/POItools_Beta01/POItools/Gameplay/BP_ViewPawn.BP_ViewPawn_C|SetSpringArm_Length_Max _poi_pawn _y)
      (Variables|/POItools_Beta01/POItools/Gameplay/BP_ViewPawn.BP_ViewPawn_C|SetSpringArm_Length_Min _poi_pawn _x))
    (:else)))