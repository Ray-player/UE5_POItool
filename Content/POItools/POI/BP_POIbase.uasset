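; Base actor for a clickable point of interest with a widget marker and a camera view baked from an editor-only spring arm, destroyed at BeginPlay.
; Clicks select it through the game mode's POI manager; selection can focus the pawn and update its zoom range.
; Widget effects (hover, brush, type, visibility) go through an interface.
; While the pawn moves, Tick scales visited markers inversely to camera arm length.
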(event Custom|ReturnPreviousPOI)

(event EventBeginPlay
  (bind _widget (Variables|Default|GetWidget))
  (bind _isbeginfocusme_ (Variables|POI属性|GetIsBeginFocusMe?))
  (bind _returnvalue (UserInterface|GetUserWidgetObject _widget))
  (Utilities|FlowControl|Sequence
    (:then_0
      (POI属性|InitPOIMessage)
      (Components|DestroyComponent (Variables|Default|GetSpringArm)))
    (:then_1
      (if (Utilities|DoesObjectImplementInterface _returnvalue "/POItools_Beta01/POItools/POI/BPI_POIWidget_Interface.BPI_POIWidget_Interface_C")
        (Variables|POI属性|SetmyPOIWidget _returnvalue)
        (CallFunction|InitPOIWidget)))
    (:then_2
      (if (> _isbeginfocusme_ 0.0)
        (Utilities|FlowControl|Delay _isbeginfocusme_)
        (CallFunction|WidgetonClicked)))))

(event Collision|EventActorBeginOverlap
  (params (OtherActor :type Actor%20Object%20Reference)))

(event EventTick
  (params (DeltaSeconds :type Float%20%28single-precision%29))
  (CallFunction|UpdataWidgetScale))

(event Custom|WidgetOnClicked
  (Default|ManagerSelectPOI (CallFunction|GetManager) self))

(event Custom|WidgetOnHovered
  ;[0.15 0.15 0.15 0.5] 选中/悬停效果
  (if (not (Variables|Default|GetisSelected))
    (if (Variables|UI设置|GetHoveredUseSelectedBrush)
      (CallFunction|ChangeSelectWidgetBrush true))
    (Class|BPIPOIWidgetInterface|PlayHoveredAni(Message) (Variables|POI属性|GetmyPOIWidget) false)))

(event Custom|Selected
  (bind _poimanager (CallFunction|GetManager))
  ;[0.15 0.15 0.15 0.5] 选中/悬停效果
  (Utilities|FlowControl|Sequence
    (:then_0
      (if (Variables|POI摄像机|GetisUpdataCameraRange)
        (Default|UpdataPawnCameraRange _poimanager (Variables|POI摄像机|GetPOI_CameraRange)))
      (if (Variables|POI属性|GetPOI_IsFocus)
        (Default|Focus (Variables|/POItools_Beta01/POItools/POI/BPC_POIManager.BPC_POIManager_C|GetPOI_Pawn _poimanager) self)))
    (:then_1
      (bind _output_get (Variables|Default|SetisSelected true))
      (CallFunction|ChangeSelectWidgetBrush _output_get)
      (Class|BPIPOIWidgetInterface|PlayHoveredAni(Message) (Variables|POI属性|GetmyPOIWidget) false)
      (Development|PrintString (Utilities|String|Append "选中层级：" (Variables|POI属性|GetPOI_Keyname))))))

(event Custom|UnSelected
  ;[0.15 0.15 0.15 0.5] 选中/悬停效果
  (bind _output_get (Variables|Default|SetisSelected false))
  (CallFunction|ChangeSelectWidgetBrush _output_get)
  (if (Variables|Default|GetisVisited)
    (Class|BPIPOIWidgetInterface|PlayHoveredAni(Message) (Variables|POI属性|GetmyPOIWidget) true)))

(event Custom|WidgetUnhovered
  ;[0.15 0.15 0.15 0.5] 选中/悬停效果
  (if (not (Variables|Default|GetisSelected))
    (if (Variables|UI设置|GetHoveredUseSelectedBrush)
      (CallFunction|ChangeSelectWidgetBrush false))
    (Class|BPIPOIWidgetInterface|PlayHoveredAni(Message) (Variables|POI属性|GetmyPOIWidget) true)))

(event EventChangePOItypes
  (params (Type :type Integer))
  (bind _mypoiwidget (Variables|POI属性|GetmyPOIWidget)
    (:then
      (Class|BPIPOIWidgetInterface|ChangeType(Message) _mypoiwidget Type false))
    (:else)))

(event EventChangePOIdata
  (params (Hid :type Boolean))
  (bind _mypoiwidget (Variables|POI属性|GetmyPOIWidget)
    (:then
      (Class|BPIPOIWidgetInterface|PlayHidDataAni(Message) _mypoiwidget Hid))
    (:else)))

(fn ConstructionScript
  (POI属性|InitPOIMessage))

(fn InitPOIMessage
  (bind _returnvalue (Transformation|GetActorLocation))
  (bind _self self)
  (bind _springarm (Variables|Default|GetSpringArm))
  (bind _cameraarmlength (Variables|POI摄像机|GetCameraArmLength))
  (bind _cameraisfollowpoi (Variables|POI摄像机|GetCameraIsFollowPOI))
  (bind _springarm_2 (Variables|Default|GetSpringArm))
  (bind _poi_camerarangeflot (Variables|POI摄像机|GetPOI_CameraRangeFlot))
  (bind _returnvalue_2 (Transformation|GetWorldRotation _springarm))
  (bind _returnvalue_3 (Utilities|GetDisplayName _self))
  (bind _returnvalue_4 (+ _cameraarmlength _poi_camerarangeflot))
  (Utilities|FlowControl|Sequence
    (:then_0
      (bind _springarm_3 (Variables|Default|GetSpringArm)
        (:then
          (Variables|/Script/Engine.SpringArmComponent|SetTargetArmLength _springarm_3 _cameraarmlength))
        (:else
          _))
      (if (> _poi_camerarangeflot 0.0)
        (Variables|POI摄像机|SetPOI_CameraRange (Utilities|Struct|MakeFloatRange (Utilities|Struct|MakeFloatRangeBound (.type (.lowerbound (Variables|POI摄像机|GetPOI_CameraRange))) (Math|Float|Clamp(Float) (- _cameraarmlength _poi_camerarangeflot) 0.0 _returnvalue_4)) (Utilities|Struct|MakeFloatRangeBound (.type (.upperbound (Variables|POI摄像机|GetPOI_CameraRange))) _returnvalue_4)))))
    (:then_1
      (if _cameraisfollowpoi
        (Variables|POI摄像机|SetCameraTrans (Math|Transform|MakeTransform _returnvalue (Transformation|GetActorRotation) "1.000000,1.000000,1.000000"))
        (else
          (Transformation|SetWorldLocation _springarm_2 (.location (Variables|POI摄像机|GetCameraTrans)) false false)
          (Transformation|SetWorldRotation _springarm_2 (.rotation (Variables|POI摄像机|GetCameraTrans)) false false))))
    (:then_2
      (Variables|POI属性|SetMyMessage (Utilities|Struct|MakeStr_POIMessage (select (Utilities|Array|IsEmpty (Variables|POI属性|GetPOI_Keyname)) _returnvalue_3 (Variables|POI属性|GetPOI_Keyname)) (select _cameraisfollowpoi _returnvalue (.location (Variables|POI摄像机|GetCameraTrans))) (Variables|POI摄像机|GetPOI_LockRotation) (.pitch _returnvalue_2) (.yaw _returnvalue_2) _cameraarmlength (Variables|POI属性|GetPOI_FocusSeconds)))
      (if (Utilities|Array|IsEmpty (Variables|POI属性|GetPOI_Keyname))
        (Variables|POI属性|SetPOI_Keyname _returnvalue_3)))))

(fn InitPOIWidget
  (Utilities|FlowControl|Sequence
    (:then_0
      (Class|BPIPOIWidgetInterface|SetPOIValue(Message) (Variables|POI属性|GetmyPOIWidget) self)
      (CallFunction|UpdataWidgetScale))
    (:then_1
      ;[0.15 0.15 0.15 0.5] 设置可视性和开场动画
      (if (Variables|POI属性|GetIsBeginHid?)
        (Rendering|SetActorHiddenInGame true)
        (Variables|Default|SetisVisited false)
        (elif (Variables|POI属性|GetHasBeginAni?)
          (POI属性|SetPOIVisit true 0.0)
          (Variables|Default|SetisVisited true))))))

(fn GetManager
  (bind _poimanager (Variables|POI属性|GetPOIManager)
    (:then
      (return _poimanager))
    (:else
      (bind _asbp_view_game_mode (Utilities|Casting|CastToBP_ViewGameMode (Game|GetGameMode)))
      (bind _output_get (Variables|POI属性|SetPOIManager (Variables|/POItools_Beta01/POItools/Gameplay/BP_ViewGameMode.BP_ViewGameMode_C|GetBPC_POIManager _asbp_view_game_mode)))
      (return _output_get))))

(fn SetPOIVisit
  (params (isVisit :type Boolean) (Delay :type Float%20%28double-precision%29))
  (Class|BPIPOIWidgetInterface|PlayVisitAni(Message) (Variables|POI属性|GetmyPOIWidget) isVisit Delay true))

(fn BindWidgetButton
  (params (Button :type Button%20Object%20Reference))
  (EventDispatchers|BindEventtoOnClicked Button (EventDispatchers|CreateEvent :!event Custom|WidgetOnClicked))
  (EventDispatchers|BindEventtoOnHovered Button (EventDispatchers|CreateEvent :!event Custom|WidgetOnHovered))
  (EventDispatchers|BindEventtoOnUnhovered Button (EventDispatchers|CreateEvent :!event Custom|WidgetUnhovered)))

(fn UpdataWidgetScale
  (bind _poimanager (CallFunction|GetManager))
  (bind _poi_widgetscalerange (Variables|POI属性|GetPOI_WidgetScaleRange))
  (bind _poi_camerarange (Variables|POI摄像机|GetPOI_CameraRange))
  (bind _poi_widgetscalerange_2 (Variables|POI属性|GetPOI_WidgetScaleRange))
  (bind _length (Default|GetpawnArmLength _poimanager))
  (bind _returnvalue (Math|Float|MapRangeClamped _length (.value (.lowerbound _poi_camerarange)) (.value (.upperbound _poi_camerarange)) (.value (.upperbound _poi_widgetscalerange)) (.value (.lowerbound _poi_widgetscalerange))))
  (if (!= (.value (.lowerbound _poi_widgetscalerange_2)) (.value (.upperbound _poi_widgetscalerange_2)))
    (if (and (Variables|Default|GetisVisited) (Default|GetPawnIsMoving _poimanager))
      (bind _mypoiwidget (Variables|POI属性|GetmyPOIWidget)
        (:then
          (bind _widget (Class|BPIPOIWidgetInterface|GetRenderWidget(Message) _mypoiwidget))
          (Utilities|IsValid _widget
            (:Is%20Valid
              (Widget|Transform|SetRenderScale _widget (Math|Vector2D|MakeVector2D _returnvalue _returnvalue)))))
        (:else)))))

(fn ChangeSelectWidgetBrush
  (params (Select :type Boolean))
  (if (Variables|UI设置|GetHasSelectedBrush)
    (Class|BPIPOIWidgetInterface|SetWidgetBrush(Message) (Variables|POI属性|GetmyPOIWidget) (select Select (Variables|UI设置|GetPOI_Widget_BrushSelected) (Variables|UI设置|GetPOI_Widget_Brush)))))

(fn GetElseMessage
  (return 0))

(fn GetIsCameraMoving?
  (return false))