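; BP_POIChangeWidget is a point-of-interest Blueprint that acts as a toggle for the POI type of the "Default" group.
; Each selection runs the parent logic, then flips a FlipFlop and asks the manager to switch that group between type indices 1 and 0, starting with 1.
; Deselection only calls the parent implementation.
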(event EventBeginPlay
  (|CallParentFunction) ; 此节点被禁用，将不会被调用。\n从引脚连出引线来编译功能。
)

(event Collision|EventActorBeginOverlap
  (params (OtherActor :type Actor%20Object%20Reference))
  (|CallParentFunction OtherActor) ; 此节点被禁用，将不会被调用。\n从引脚连出引线来编译功能。
)

(event EventTick
  (params (DeltaSeconds :type Float%20%28single-precision%29))
  (|CallParentFunction DeltaSeconds) ; 此节点被禁用，将不会被调用。\n从引脚连出引线来编译功能。
)

(event EventSelected
  (|CallParentFunction)
  (bind _isa (Utilities|FlowControl|FlipFlop)
    (:A
      _)
    (:B
      _))
  (Default|ChangeGroupsPOItype (CallFunction|GetManager) "Default" (select _isa 1 0)))

(event EventUnSelected
  (|CallParentFunction))

(fn ConstructionScript
  (|CallParentFunction))