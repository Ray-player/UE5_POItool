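; BP_ViewPawn is a mouse-driven orbit camera pawn for viewing and focusing on points of interest (POI).
; Enhanced Input drives left-drag rotation with clamped pitch, right-drag panning and wheel zoom, with curves scaling pan and zoom by normalized spring arm length.
; Focus calls play a timeline blending location, rotation and arm length toward POI data, then notify the target.
; Tick smooths arm length, and the original camera state is saved once on possession.
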(event Custom|ArmSmooth
  (params (DeltaTime :type Float%20%28double-precision%29))
  (bind _springarm (Variables|Default|GetSpringArm))
  ;[0.15 0.15 0.15 0.5] 鼠标操作
  ;;[0.15 0.15 0.15 0.5] 滚轮放缩
  (if (Math|Float|NearlyEqual(Float) (Variables|放缩|GetNewTargetArmLength) (Variables|/Script/Engine.SpringArmComponent|GetTargetArmLength _springarm) (Variables|放缩|GetSpringArm_NearTolerance))
    (Variables|Default|SetisCloseArm true)
    (else
      (Variables|/Script/Engine.SpringArmComponent|SetTargetArmLength _springarm (Math|Interpolation|FInterpTo (Variables|/Script/Engine.SpringArmComponent|GetTargetArmLength _springarm) (Variables|放缩|GetNewTargetArmLength) DeltaTime (Variables|放缩|GetFocusZoomSpeed)))
      (Variables|Default|SetisCloseArm (Math|Float|NearlyEqual(Float) (Variables|放缩|GetNewTargetArmLength) (Variables|/Script/Engine.SpringArmComponent|GetTargetArmLength _springarm) (Variables|放缩|GetSpringArm_NearTolerance)))))
  (if (Variables|Default|GetisCloseArm)
    (Default|CallCloseArmComplete)))

(event Custom|Focus
  (params (POItarget :type BP%20PO%20Ibase%20Object%20Reference))
  ;[1 1 1] Focus POI
  (if (Variables|Default|GetIsFocusEnd)
    (Variables|Default|SetCurrentPOItarget POItarget)
    (CallFunction|FocusbyData (Variables|/POItools_Beta01/POItools/POI/BP_POIbase.BP_POIbase_C|GetMyMessage POItarget))))

(event Custom|FocusArmLength
  (params (NewArmLength :type Float%20%28double-precision%29))
  ;[0.15 0.15 0.15 0.5] 鼠标操作
  ;;[0.15 0.15 0.15 0.5] 滚轮放缩
  (Variables|放缩|SetNewTargetArmLength NewArmLength)
  (Variables|Default|SetisCloseArm (Math|Float|NearlyEqual(Float) (Variables|/Script/Engine.SpringArmComponent|GetTargetArmLength (Variables|Default|GetSpringArm)) (Variables|放缩|GetNewTargetArmLength) (Variables|放缩|GetSpringArm_NearTolerance))))

(event Custom|FocusByData
  (params (StrMes :type Str%20POI%20Message%20Structure))
  (bind (_name _poi_location _lockpotation _poi_pitch _poi_yaw _poi_armlength _poi_focusseconds) (Utilities|Struct|BreakStr_POIMessage StrMes))
  (bind _self self)
  (bind _returnvalue (Pawn|GetControlRotation _self :!class /Script/Engine.Pawn))
  ;[1 1 1] Focus POI
  (Variables|Default|SetIsFocusEnd false)
  (Utilities|FlowControl|Sequence
    (:then_0
      (if (> _poi_armlength 0.0)
        (CallFunction|FocusArmLength _poi_armlength)))
    (:then_1
      (Variables|Default|SetLocation_Current (Transformation|GetActorLocation))
      (Variables|Default|SetPitch_Current (.pitch _returnvalue))
      (Variables|Default|SetYaw_Current (.yaw _returnvalue)))
    (:then_2
      (Components|Timeline|SetPlayRate (Variables|Default|GetFocusLine) (/ 1.0 (Math|Float|Clamp(Float) _poi_focusseconds 0.01 999999.0)))
      (bind _outdata (Timeline|FocusLine PlayFromStart)
        (:Update
          (Transformation|SetActorLocation (Math|Vector|Lerp(Vector) (Variables|Default|GetLocation_Current) _poi_location _outdata) false false)
          (if (not _lockpotation)
            (Pawn|SetControlRotation (Game|GetPlayerController 0) (Math|Rotator|Lerp(Rotator) (Math|Rotator|MakeRotator 0.0 (Variables|Default|GetPitch_Current) (Variables|Default|GetYaw_Current)) (Math|Rotator|MakeRotator 0.0 _poi_pitch _poi_yaw) _outdata true))))
        (:Finished
          (Variables|Default|SetIsFocusEnd true)
          (bind _currentpoitarget (Variables|Default|GetCurrentPOItarget)
            (:then
              (Default|UpdateMouseMoveandZoom _currentpoitarget)
              (Variables|Default|SetCurrentPOItarget 0))
            (:else)))))))

(event Custom|OnOffInput
  (params (Off :type Boolean))
  (bind _returnvalue (Game|GetPlayerController 0))
  (bind _returnvalue_2 (PlayerController|LocalPlayerSubsystems|GetEnhancedInputLocalPlayerSubsystem _returnvalue))
  ;[0.15 0.15 0.15 0.5] Input
  (if Off
    (Input|RemoveMappingContext _returnvalue_2 "/POItools_Beta01/POItools/Input/IMC_Control.IMC_Control" "(bIgnoreAllPressedKeysUntilRelease=True,bForceImmediately=False,bNotifyUserSettings=False)")
    (else
      (Input|AddMappingContext _returnvalue_2 "/POItools_Beta01/POItools/Input/IMC_Control.IMC_Control" 0 "(bIgnoreAllPressedKeysUntilRelease=True,bForceImmediately=False,bNotifyUserSettings=False)"))))

(event Input|EnhancedActionEvents|EnhancedInputActionIA_MouseLeft
  (params (ActionValue :type Boolean) (ElapsedSeconds :type Float%20%28double-precision%29) (TriggeredSeconds :type Float%20%28double-precision%29) (InputAction :type Input%20Action%20Object%20Reference :default "/POItools_Beta01/POItools/Input/IA_MouseLeft.IA_MouseLeft"))
  ;[0.15 0.15 0.15 0.5] 鼠标操作
  ;;[0.15 0.15 0.15 0.5] 左右键按压判断
  (:Started
    (Variables|平移|SetLeftIsPressed true))
  (:Completed
    (Variables|平移|SetLeftIsPressed false)))

(event Input|EnhancedActionEvents|EnhancedInputActionIA_MouseXY
  (params (ActionValue :type Vector%202D%20Structure) (ElapsedSeconds :type Float%20%28double-precision%29) (TriggeredSeconds :type Float%20%28double-precision%29) (InputAction :type Input%20Action%20Object%20Reference :default "/POItools_Beta01/POItools/Input/IA_MouseXY.IA_MouseXY"))
  (bind _returnvalue (CallFunction|SpringArmLengthNormalized))
  (bind _returnvalue_2 (Pawn|GetControlRotation :!class /Script/Engine.Pawn))
  (bind _pan_curve (Variables|平移|GetPan_Curve))
  (bind _panmovespeed (Variables|平移|GetPanMoveSpeed))
  (bind _returnvalue_3 (Math|Curves|GetFloatValue _pan_curve _returnvalue))
  (bind _returnvalue_4 (* _returnvalue_3 _panmovespeed))
  ;[0.15 0.15 0.15 0.5] 鼠标操作
  (Utilities|FlowControl|Sequence
    (:then_0
      ;;[0.15 0.15 0.15 0.5] 左键旋转
      (if (and (Variables|旋转|GetisUseRotation?) (Variables|平移|GetLeftIsPressed))
        (Pawn|SetControlRotation (Game|GetPlayerController 0) (Math|Rotator|MakeRotator 0.0 (CallFunction|GetRotationValue (.y ActionValue) false) (CallFunction|GetRotationValue (.x ActionValue) true)))))
    (:then_1
      ;;[0.15 0.15 0.15 0.5] 鼠标右键移动
      (if (and (Variables|平移|GetRightIsPressed) (Variables|平移|GetisUsePan?))
        (Pawn|Input|AddMovementInput (Math|Vector|GetRightVector (Math|Rotator|MakeRotator (.roll _returnvalue_2) 0.0 (.yaw _returnvalue_2))) (* (.x ActionValue) _returnvalue_4) false)
        (Pawn|Input|AddMovementInput (Math|Vector|GetForwardVector (Math|Rotator|MakeRotator 0.0 0.0 (.yaw (Pawn|GetControlRotation :!class /Script/Engine.Pawn)))) (* (.y ActionValue) _returnvalue_4) false)))))

(event Input|EnhancedActionEvents|EnhancedInputActionIA_MouseRight
  (params (ActionValue :type Boolean) (ElapsedSeconds :type Float%20%28double-precision%29) (TriggeredSeconds :type Float%20%28double-precision%29) (InputAction :type Input%20Action%20Object%20Reference :default "/POItools_Beta01/POItools/Input/IA_MouseRight.IA_MouseRight"))
  ;[0.15 0.15 0.15 0.5] 鼠标操作
  ;;[0.15 0.15 0.15 0.5] 左右键按压判断
  (:Started
    (Variables|平移|SetRightIsPressed true))
  (:Completed
    (Variables|平移|SetRightIsPressed false)))

(event Input|EnhancedActionEvents|EnhancedInputActionIA_MouseWheel
  (params (ActionValue :type Float%20%28double-precision%29) (ElapsedSeconds :type Float%20%28double-precision%29) (TriggeredSeconds :type Float%20%28double-precision%29) (InputAction :type Input%20Action%20Object%20Reference :default "/POItools_Beta01/POItools/Input/IA_MouseWheel.IA_MouseWheel"))
  ;[0.15 0.15 0.15 0.5] 鼠标操作
  ;;[0.15 0.15 0.15 0.5] 滚轮放缩
  (Variables|放缩|SetNewTargetArmLength (Math|Float|Clamp(Float) (+ (Variables|/Script/Engine.SpringArmComponent|GetTargetArmLength (Variables|Default|GetSpringArm)) (* -1.0 (Variables|放缩|GetZoom_Speed_Mouse) ActionValue (Math|Curves|GetFloatValue (Variables|放缩|GetZoom_Intensity_Curve) (CallFunction|SpringArmLengthNormalized)))) (Variables|放缩|GetSpringArm_Length_Min) (Variables|放缩|GetSpringArm_Length_Max)))
  (Variables|Default|SetisCloseArm (Math|Float|NearlyEqual(Float) (Variables|/Script/Engine.SpringArmComponent|GetTargetArmLength (Variables|Default|GetSpringArm)) (Variables|放缩|GetNewTargetArmLength) (Variables|放缩|GetSpringArm_NearTolerance))))

(event EventBeginPlay)

(event Collision|EventActorBeginOverlap
  (params (OtherActor :type Actor%20Object%20Reference)))

(event EventControllerChanged
  (params (OldController :type Controller%20Object%20Reference) (NewController :type Controller%20Object%20Reference))
  (bind _returnvalue (Game|GetPlayerController 0))
  (bind _returnvalue_2 (PlayerController|LocalPlayerSubsystems|GetEnhancedInputLocalPlayerSubsystem _returnvalue))
  ;[0.15 0.15 0.15 0.5] Input
  (Variables|放缩|SetNewTargetArmLength (Variables|/Script/Engine.SpringArmComponent|GetTargetArmLength (Variables|Default|GetSpringArm)))
  (Utilities|FlowControl|Sequence
    (:then_0
      (Utilities|FlowControl|DoOnce false
        (:Completed
          (CallFunction|SaveOriginCameraData))))
    (:then_1
      (Input|AddMappingContext _returnvalue_2 "/POItools_Beta01/POItools/Input/IMC_Control.IMC_Control" 0 "(bIgnoreAllPressedKeysUntilRelease=True,bForceImmediately=False,bNotifyUserSettings=False)")
      (Input|AddMappingContext _returnvalue_2 "/POItools_Beta01/POItools/Input/IMC_Click.IMC_Click" 1 "(bIgnoreAllPressedKeysUntilRelease=True,bForceImmediately=False,bNotifyUserSettings=False)"))))

(event EventTick
  (params (DeltaSeconds :type Float%20%28single-precision%29))
  ;[0.15 0.15 0.15 0.5] 鼠标操作
  ;;[0.15 0.15 0.15 0.5] 滚轮放缩
  (if (not (Variables|Default|GetisCloseArm))
    (CallFunction|ArmSmooth DeltaSeconds)))

(fn ConstructionScript)

(fn SpringArmLengthNormalized
  (return (Math|Float|NormalizetoRange (Variables|/Script/Engine.SpringArmComponent|GetTargetArmLength (Variables|Default|GetSpringArm)) (Variables|放缩|GetSpringArm_Length_Min) (Variables|放缩|GetSpringArm_Length_Max))))

(fn GetRotationValue
  (params (Rotate :type Float%20%28double-precision%29) (isYaw :type Boolean))
  (bind _returnvalue (Game|GetPlayerController 0))
  (bind _rotation_speed_mouse (Variables|旋转|GetRotation_Speed_Mouse))
  (bind _returnvalue_2 (Pawn|GetControlRotation _returnvalue :!class /Script/Engine.Controller))
  (bind _returnvalue_3 (* _rotation_speed_mouse Rotate))
  (return (Math|Float|SelectFloat (+ _returnvalue_3 (.yaw _returnvalue_2)) (Math|Float|ClampAngle (+ (.pitch _returnvalue_2) _returnvalue_3) (Variables|旋转|GetPitchLimit_Min) (Variables|旋转|GetPitchLimit_Max)) isYaw)))

(fn SaveOriginCameraData
  (bind _self self)
  (bind _returnvalue (Transformation|GetActorRotation _self))
  (Variables|Default|SetOriginCameraData (Utilities|Struct|MakeStr_POIMessage "Pawn" (Transformation|GetActorLocation _self) false (.pitch _returnvalue) (.yaw _returnvalue) (Variables|/Script/Engine.SpringArmComponent|GetTargetArmLength (Variables|Default|GetSpringArm)) 1.0)))